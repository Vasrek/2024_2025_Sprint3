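; BP_MasterInteract is an interactable object, apparently a base class, that signals when the player is in range.
; While usable, its sphere overlap adds or hides the interact widget on BP_Player and shows or hides an arrow.
; Two timelines restart each other to bob the arrow up and down by relative Z offsets.
; The construction script sizes the sphere from InteractRange, and RemoveArrow hides the arrow directly.
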(event OnComponentBeginOverlap(InteractSphereCol)
  (params (OverlappedComponent :type Primitive%20Component%20Object%20Reference) (OtherActor :type Actor%20Object%20Reference) (OtherComp :type Primitive%20Component%20Object%20Reference) (OtherBodyIndex :type Integer) (bFromSweep :type Boolean) (SweepResult :type Hit%20Result%20Structure%20%28by%20ref%29))
  (if (Variables|Default|GetbCanBeUsed?)
    (bind _asbp_player (Utilities|Casting|CastToBP_Player OtherActor))
    (Default|AddInteractWidget _asbp_player self)
    (Utilities|IsValid (Variables|Default|GetArrow)
      (:Is%20Valid
        (Development|SetHiddeninGame (Variables|Default|GetArrow) false false)
        (CallFunction|GoUpArrow)))))

(event OnComponentEndOverlap(InteractSphereCol)
  (params (OverlappedComponent :type Primitive%20Component%20Object%20Reference) (OtherActor :type Actor%20Object%20Reference) (OtherComp :type Primitive%20Component%20Object%20Reference) (OtherBodyIndex :type Integer))
  (if (Variables|Default|GetbCanBeUsed?)
    (bind _asbp_player (Utilities|Casting|CastToBP_Player OtherActor))
    (Default|HideInteractWidget _asbp_player)
    (Utilities|IsValid (Variables|Default|GetArrow)
      (:Is%20Valid
        (Development|SetHiddeninGame (Variables|Default|GetArrow) true false)))))

(event Custom|GoDownArrow
  (bind _arrow (Variables|Default|GetArrow))
  (bind _relativelocation (Variables|/Script/Engine.SceneComponent|GetRelativeLocation _arrow))
  (bind _zpos (Timeline|DownArrow PlayFromStart)
    (:Update
      (Transformation|SetRelativeLocation _arrow (Math|Vector|MakeVector (.x _relativelocation) (.y _relativelocation) (- (.z _relativelocation) _zpos)) false false))
    (:Finished
      (CallFunction|GoUpArrow))))

(event Custom|RemoveArrow
  (Utilities|IsValid (Variables|Default|GetArrow)
    (:Is%20Valid
      (Development|SetHiddeninGame (Variables|Default|GetArrow) true false))))

(event Custom|GoUpArrow
  (bind _arrow (Variables|Default|GetArrow))
  (bind _relativelocation (Variables|/Script/Engine.SceneComponent|GetRelativeLocation _arrow))
  (bind _zpos (Timeline|UpArrow PlayFromStart)
    (:Update
      (Transformation|SetRelativeLocation _arrow (Math|Vector|MakeVector (.x _relativelocation) (.y _relativelocation) (+ (.z _relativelocation) _zpos)) false false))
    (:Finished
      (CallFunction|GoDownArrow))))

(event EventBeginPlay)

(fn ConstructionScript
  (Components|Sphere|SetSphereRadius (Variables|Default|GetInteractSphereCol) (Variables|Default|GetInteractRange) true))