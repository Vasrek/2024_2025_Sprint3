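; BP_MasterDoor is a base interactable door that animates its InteractMesh for successful and failed opening attempts.
; GoodOpenDoor plays the OpenDoor timeline to swing the mesh open by driving its relative yaw.
; WrongOpenDoor plays the DontHaveKey timeline on the same yaw as locked-door feedback, only when KeyToOpen is valid.
; Both restart from the beginning and feed the mesh's world roll and pitch into the relative rotation.
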(event Custom|WrongOpenDoor
  (bind _interactmesh (Variables|Default|GetInteractMesh))
  (bind _returnvalue (Transformation|GetWorldRotation _interactmesh))
  (Utilities|IsValid (Variables|Default|GetKeyToOpen)
    (:Is%20Valid
      (bind _rotdoor (Timeline|DontHaveKey PlayFromStart)
        (:Update
          (Transformation|SetRelativeRotation (Variables|Default|GetInteractMesh) (Math|Rotator|MakeRotator (.roll _returnvalue) (.pitch _returnvalue) _rotdoor) false false))))))

(event Custom|GoodOpenDoor
  (bind _interactmesh (Variables|Default|GetInteractMesh))
  (bind _returnvalue (Transformation|GetWorldRotation _interactmesh))
  (bind _opendoorrot (Timeline|OpenDoor PlayFromStart)
    (:Update
      (Transformation|SetRelativeRotation (Variables|Default|GetInteractMesh) (Math|Rotator|MakeRotator (.roll _returnvalue) (.pitch _returnvalue) _opendoorrot) false false))))

(event EventBeginPlay
  (|CallParentFunction) ; This node is disabled and will not be called.\nDrag off pins to build functionality.
)

(fn ConstructionScript
  (|CallParentFunction))